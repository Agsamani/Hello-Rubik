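; Playable Rubik's Cube actor that builds 27 BP_Cubie child actors and turns slices, or the whole cube with Shift, by mouse drag.
; Hit normal and initial drag direction choose the axis.
; RotateGroup temporarily attaches matching cubies to a pivot to rotate them, with glow feedback.
; Release snaps to 90 degrees via timeline, then rebuilds indices from world positions and changes the background color.
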(event `self.ReceiveBeginPlay`
  (`self.EnableInput` (`GameplayStatics.GetPlayerController` 0)))

(event `self.ReceiveTick`
  (params (DeltaSeconds :type "Float (single-precision)"))
  (if (and (`self.Selected`) (not (`self.Animating`)))
    (bind _angle (`self.CalculateAngle` (`self.InitialMousePos`)))
    (bind _rotatedcubes (`self.RotateGroup` (`self.SelectedAxis`) (`self.SelectedIndex`) _angle (`self.RotateWhole`)))
    (set `self.RotationAmount` _angle)
    (if (and (not (`self.IsGlowing`)) (not (`self.ParamsNotCalculated`)))
      (set `self.IsGlowing` true)
      (`self.StartGlowing` _rotatedcubes))))

(event `EnhancedInput|/Game/IA_R`
  (params (ActionValue :type Boolean) (ElapsedSeconds :type "Float (double-precision)") (TriggeredSeconds :type "Float (double-precision)") (InputAction :type "InputAction Object Reference" :default "/Game/IA_R.IA_R")))

(event `OnSnap`
  (params (AmountBase :type "Float (double-precision)") (AmountTraget :type "Float (double-precision)"))
  (set `self.Animating` true)
  (bind (_direction _amountalpha _emissionintensity) (`Timeline|RotationSnapTimeline` :!via `PlayFromStart`)
    (:`Update`
      (bind _rotatedcubes (`self.RotateGroup` (`self.SelectedAxis`) (`self.SelectedIndex`) (`KismetMathLibrary.Lerp` AmountBase AmountTraget _amountalpha) (`self.RotateWhole`)))
      (for _array_element _rotatedcubes
        (if (`self.IsGlowing`)
          (`/Game/BP_Cubie.SetMaterialEmission` _array_element _emissionintensity))))
    (:`Finished`
      (`GameplayStatics.PlaySound2D` "/Game/Sounds/switch13.switch13" 1.0 1.0 0.0 null null)
      (set `self.Animating` false)
      (set `self.Selected` false)
      (set `self.IsGlowing` false)
      (set `self.InitialMousePos` (0.0 0.0 0.0))
      (set `self.SelectedIndex` 0)
      (set `self.ParamsNotCalculated` true)
      (`SceneComponent.K2_SetRelativeRotation` :`self` (`self.RotationGroup`))
      (set `self.RotationAmount` 0.0)
      (`self.AssignIndices`)
      (set `self.SelectedCubie` null)
      (set `self.RotateWhole` false)
      (bind _returnvalue (`GameplayStatics.GetActorOfClass` "/Game/BP_Background.BP_Background_C"))
      (`/Game/BP_Background.ChangeColor` _returnvalue))))

(event `EnhancedInput|/Game/IA_MouseMove`
  (params (ActionValue :type "Vector2D Structure") (ElapsedSeconds :type "Float (double-precision)") (TriggeredSeconds :type "Float (double-precision)") (InputAction :type "InputAction Object Reference" :default "/Game/IA_MouseMove.IA_MouseMove"))
  (:`Triggered`
    (bind _output_get (set `self.InitialMousePos` (+ (`self.InitialMousePos`) ActionValue)))
    (`self.CalculateAngle` _output_get)))

(event `EnhancedInput|/Game/IA_RotatePart`
  (params (ActionValue :type Boolean) (ElapsedSeconds :type "Float (double-precision)") (TriggeredSeconds :type "Float (double-precision)") (InputAction :type "InputAction Object Reference" :default "/Game/IA_RotatePart.IA_RotatePart"))
  (bind (_bblockinghit _binitialoverlap _time _distance _location _impactpoint _normal _impactnormal _physmat _hitactor) (`GameplayStatics.BreakHitResult` (`PlayerController.GetHitResultUnderCursorByChannel` (`GameplayStatics.GetPlayerController` 0) "TraceTypeQuery1" true)))
  (:`Triggered`
    (if (not (`self.Animating`))
      (set `self.RotationAmount` 0.0)
      (if (not (`self.Selected`))
        (set `self.InitialMousePos` (0.0 0.0 0.0))
        (set `self.RotateWhole` false)
        (bind _asbp_cubie (cast `/Game/BP_Cubie` _hitactor)
          (:`then`
            (set `self.CubeHit` true)
            (if (`PlayerController.IsInputKeyDown` (`GameplayStatics.GetPlayerController` 0) "LeftShift")
              (set `self.RotateWhole` true))
            (set `self.SelectedCubie` _asbp_cubie)
            (set `self.SelectedNormale` _normal)
            (set `self.Selected` true)
            (`GameplayStatics.PlaySound2D` "/Game/Sounds/click2.click2" 1.5 1.0 0.0 null null))
          (:`CastFailed`
            (set `self.CubeHit` false))))))
  (:`Canceled`
    (if (`self.CubeHit`) :!label _label
      (`self.SnapRotation`)
      (set `self.CubeHit` false)))
  (:`Completed`
    (goto _label)))

(event `StartGlowing`
  (params (CubiesToGLow :type "Array of /Game/BP_Cubie Object Reference"))
  (bind (_direction _newtrack_0) (`Timeline|GlowTimeline` :!via `PlayFromStart`)
    (:`Update`
      (for _array_element CubiesToGLow
        (`/Game/BP_Cubie.SetMaterialEmission` _array_element _newtrack_0)))))

(fn `AssignIndices`
  (for _array_element (`self.CubieArray`)
    (bind _cubeindex (`/Game/BP_Cubie.CubeIndex` _array_element))
    (bind (_x _y _z) (break `IntVector` (`KismetMathLibrary.FTruncVector` (/ (+ (- (`SceneComponent.K2_GetComponentLocation` (`Actor.RootComponent` _array_element)) (`SceneComponent.K2_GetComponentLocation` (`self.DefaultSceneRoot`))) (201.0 201.0 201.0)) (200.0 200.0 200.0)))))
    (`KismetArrayLibrary.Array_Set` _cubeindex 0 _x)
    (`KismetArrayLibrary.Array_Set` _cubeindex 1 _y)
    (`KismetArrayLibrary.Array_Set` _cubeindex 2 _z)))

(fn `AutoRotate`)

(fn `CalculateAngle`
  (params (DistVec :type "Vector Structure"))
  (returns (Angle :type "Float (double-precision)"))
  (bind _x (.x DistVec))
  (bind _y (.y DistVec))
  (bind _invrotationspeed (`self.InvRotationSpeed`))
  (if (and (< (`KismetMathLibrary.VSize` DistVec) (`self.DistThresh`)) (`self.ParamsNotCalculated`))
    (`self.CalculateAxisAndIndex` (> (`KismetMathLibrary.Abs` _x) (`KismetMathLibrary.Abs` _y)))
    (return 0.0)
    (else
      (set `self.ParamsNotCalculated` false)
      (if (== (`self.SelectedIndex`) 2)
        (return (/ _x _invrotationspeed))
        (else
          (return (/ _y _invrotationspeed)))))))

(fn `CalculateAxisAndIndex`
  (params (IsHorizontal :type Boolean))
  (bind _selectedcubie (`self.SelectedCubie`))
  (if IsHorizontal
    (set `self.SelectedIndex` 2)
    (elif (> (`KismetMathLibrary.Dot_VectorVector` (`self.SelectedNormale`) (1.0 0.0 0.0)) (`KismetMathLibrary.Dot_VectorVector` (`self.SelectedNormale`) (0.0 1.0 0.0)))
      (set `self.SelectedIndex` 1)
      (else
        (set `self.SelectedIndex` 0))))
  (if (`KismetSystemLibrary.IsValid` _selectedcubie)
    (set `self.SelectedAxis` (`|GetArrayItem` (`/Game/BP_Cubie.CubeIndex` _selectedcubie) (`self.SelectedIndex`)))))

(fn `RotateGroup`
  (params (Axis :type Integer) (Index :type Integer) (Amount :type "Float (double-precision)") (RotateWholeCube :type Boolean :default false))
  (returns (RotatedCubes :type "Array of /Game/BP_Cubie Object Reference"))
  (locals (RotatedCubies :type "Array of /Game/BP_Cubie Object Reference"))
  (bind _rotatedcubies (`local.RotatedCubies`))
  (`KismetArrayLibrary.Array_Clear` (`local.RotatedCubies`))
  (set `self.RotationCenterPos` (0.0 0.0 0.0))
  (for _array_element (`self.CubieArray`)
    (if (or (== (`|GetArrayItem` (`/Game/BP_Cubie.CubeIndex` _array_element) Index) Axis) RotateWholeCube)
      (bind _rootcomponent (`Actor.RootComponent` _array_element))
      (`SceneComponent.K2_AttachToComponent` _rootcomponent (`self.RotationGroup`) "None" "KeepWorld" "KeepWorld" "KeepWorld" true)
      (set `self.RotationCenterPos` (+ (`self.RotationCenterPos`) (`SceneComponent.K2_GetComponentLocation` _rootcomponent)))
      (`KismetArrayLibrary.Array_Add` _rotatedcubies _array_element)))
  (if (== Index 0)
    (`KismetMathLibrary.Vector_Set` (`self.RotationAxisBase`) -1.0)
    (`SceneComponent.K2_SetRelativeRotation` (`self.RotationGroup`) (`KismetMathLibrary.MakeRotator` (.x (* (`self.RotationAxisBase`) Amount)) (.y (* (`self.RotationAxisBase`) Amount)) (.z (* (`self.RotationAxisBase`) Amount))) false false :!label _label)
    (for _array_element_2 (`self.CubieArray`)
      (if (or (== (`|GetArrayItem` (`/Game/BP_Cubie.CubeIndex` _array_element_2) Index) Axis) RotateWholeCube)
        (`SceneComponent.K2_DetachFromComponent` (`Actor.RootComponent` _array_element_2) "KeepWorld" "KeepWorld" "KeepWorld" true)))
    (return _rotatedcubies)
    (elif (== Index 1)
      (`KismetMathLibrary.Vector_Set` (`self.RotationAxisBase`) 0.0 1.0)
      (goto _label)
      (elif (== Index 2)
        (`KismetMathLibrary.Vector_Set` (`self.RotationAxisBase`) 0.0 0.0 -1.0)
        (goto _label)))))

(fn `SnapRotation`
  (bind _rotationamount (`self.RotationAmount`))
  (`self.OnSnap` _rotationamount (`KismetMathLibrary.Conv_IntToDouble` (* (`KismetMathLibrary.Round` (/ _rotationamount 90.0)) 90))))

(fn `UserConstructionScript`
  (for _index (range 27)
    (bind _returnvalue (`AddComponent|NODE_AddChildActorComponent-1`))
    (bind _returnvalue_2 (mod _index 3))
    (bind _returnvalue_3 (/ _index 3))
    (bind _returnvalue_4 (mod _returnvalue_3 3))
    (bind _returnvalue_5 (mod (/ _returnvalue_3 3) 3))
    (`SceneComponent.K2_SetRelativeTransform` _returnvalue (`KismetMathLibrary.MakeTransform` (- (* (`KismetMathLibrary.MakeVector` (`KismetMathLibrary.Conv_IntToDouble` _returnvalue_2) (`KismetMathLibrary.Conv_IntToDouble` _returnvalue_4) (`KismetMathLibrary.Conv_IntToDouble` _returnvalue_5)) (200.0 200.0 200.0)) (200.0 200.0 200.0)) (struct) (0.93 0.93 0.93)) false false)
    (bind _asbp_cubie (cast `/Game/BP_Cubie` (`ChildActorComponent.ChildActor` _returnvalue)))
    (`KismetArrayLibrary.Array_Add` (`self.CubieArray`) _asbp_cubie)
    (bind _array (`|MakeArray` _returnvalue_2 _returnvalue_4 _returnvalue_5))
    (set `/Game/BP_Cubie.CubeIndex` _array _asbp_cubie)
    (set `/Game/BP_Cubie.InitCubeIndex` _array _asbp_cubie)
    (`/Game/BP_Cubie.AddSides` _asbp_cubie)))