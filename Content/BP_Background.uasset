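; Background plane actor that crossfades between random colors from DT_ColorTable.
; Construction creates a dynamic MT_BG material and sets both color parameters to one random table color.
; ChangeColor ignores calls during a fade, picks a color differing from the last, and writes it to alternating slots.
; A timeline then drives BlendAlpha forward or inverted, while an unused construction branch would scatter wireframe meshes on a sphere.
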(event `OnColorChange`
  (bind _bgmat (`self.bgMat`))
  (set `self.IsChanging` true)
  (bind (_direction _alpha) (`Timeline|BlendAlphaTimeline` :!via `PlayFromStart`)
    (:`Update`
      (if (`self.Turn`)
        (`MaterialInstanceDynamic.SetScalarParameterValue` _bgmat "BlendAlpha" (- 1.0 _alpha))
        (else
          (`MaterialInstanceDynamic.SetScalarParameterValue` _bgmat "BlendAlpha" _alpha))))
    (:`Finished`
      (set `self.IsChanging` false))))

(fn `ChangeColor`
  (bind _bgmat (`self.bgMat`))
  (bind _selectedcolor (`self.SelectedColor`))
  (if (not (`self.IsChanging`))
    (bind _color (`self.GetRandomColor`))
    (set `self.SelectedColor` _color)
    (while (== (`self.PrevColor`) (`self.SelectedColor`))
      (bind _color_2 (`self.GetRandomColor`))
      (set `self.SelectedColor` _color_2))
    (if (`self.Turn`)
      (`MaterialInstanceDynamic.SetVectorParameterValue` _bgmat "Color2" _selectedcolor)
      (else
        (`MaterialInstanceDynamic.SetVectorParameterValue` _bgmat "Color1" _selectedcolor)))
    (set `self.Turn` (xor (`self.Turn`) true))
    (set `self.PrevColor` _selectedcolor)
    (`self.OnColorChange`)))

(fn `GetRandomColor`
  (returns (Color :type "LinearColor Structure"))
  (bind _outrownames (`DataTableFunctionLibrary.GetDataTableRowNames` "/Game/DT_ColorTable.DT_ColorTable"))
  (bind _returnvalue (`|GetDataTableRow` "/Game/DT_ColorTable.DT_ColorTable" (`|GetArrayItem` _outrownames (`KismetMathLibrary.RandomInteger` (`KismetArrayLibrary.Array_Length` _outrownames))))
    (:`then`
      _)
    (:`RowNotFound`
      _))
  (return (`.Color_2_CFD72002491B7286ABA2E1915FB5A22F` (break `/Game/S_SideColor` _returnvalue))))

(fn `GetRandomSpherePoint`
  (returns (Point :type "Vector Structure"))
  (bind _returnvalue (* (`KismetMathLibrary.MultiplyByPi` (`KismetMathLibrary.RandomFloat`)) 1.0))
  (bind _returnvalue_2 (`KismetMathLibrary.Acos` (- (* (`KismetMathLibrary.RandomFloat`) 2.0) 1.0)))
  (bind _returnvalue_3 (`KismetMathLibrary.Sin` _returnvalue_2))
  (return (`KismetMathLibrary.MakeVector` (* (`KismetMathLibrary.Sin` _returnvalue) _returnvalue_3) (* (`KismetMathLibrary.Cos` _returnvalue) _returnvalue_3) (`KismetMathLibrary.Cos` _returnvalue_2))))

(fn `UserConstructionScript`
  (bind _plane (`self.Plane`))
  (bind _returnvalue (`PrimitiveComponent.CreateDynamicMaterialInstance` _plane 0 "/Game/MT_BG.MT_BG" "None"))
  (`PrimitiveComponent.SetMaterial` _plane 0 _returnvalue)
  (bind _outrownames (`DataTableFunctionLibrary.GetDataTableRowNames` "/Game/DT_ColorTable.DT_ColorTable"))
  (bind _returnvalue_2 (`|GetDataTableRow` "/Game/DT_ColorTable.DT_ColorTable" (`|GetArrayItem` _outrownames (`KismetMathLibrary.RandomInteger` (`KismetArrayLibrary.Array_Length` _outrownames))))
    (:`then`
      (bind _color (break `/Game/S_SideColor` _returnvalue_2))
      (`MaterialInstanceDynamic.SetVectorParameterValue` _returnvalue "Color1" _color)
      (`MaterialInstanceDynamic.SetVectorParameterValue` _returnvalue "Color2" _color)
      (set `self.bgMat` _returnvalue))))