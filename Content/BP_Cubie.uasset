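; Single cubie of a Rubik's-style cube that builds its own colored stickers for the outward-facing sides.
; AddSides checks each axis of InitCubeIndex and, at either outer layer, adds a Cubie_seg mesh with a dynamic MT_Side material colored from DT_ColorTable.
; Those materials collect in SideMaterials, which SetMaterialEmission uses to set a scaled glow intensity on all stickers.
; BeginPlay separately gives the cubie body a black dynamic material.
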(event `self.ReceiveBeginPlay`
  (bind _returnvalue (`PrimitiveComponent.CreateDynamicMaterialInstance` (`self.Cubie_Mesh`) 0 "/Game/MT_BasicCubie.MT_BasicCubie" "None"))
  (`MaterialInstanceDynamic.SetVectorParameterValue` _returnvalue "Color" (`KismetMathLibrary.MakeColor` 0.0 0.0 0.0 0.0)))

(fn `AddSides`
  (bind _initcubeindex (`self.InitCubeIndex`))
  (switch `int` (`|GetArrayItem` _initcubeindex)
    (:`0`
      (bind _returnvalue (`AddComponent|NODE_AddStaticMeshComponent-0`))
      (`StaticMeshComponent.SetStaticMesh` _returnvalue "/Game/Meshes/cubie_seg.cubie_seg")
      (`SceneComponent.K2_SetRelativeTransform` _returnvalue (`KismetMathLibrary.MakeTransform` (-100.0 0.0 0.0) (struct :`Pitch` 90.0) (0.86 0.86 0.86)) false false)
      (bind _returnvalue_2 (`PrimitiveComponent.CreateDynamicMaterialInstance` _returnvalue 0 "/Game/MT_Side.MT_Side" "None"))
      (`KismetArrayLibrary.Array_Add` (`self.SideMaterials`) _returnvalue_2)
      (`PrimitiveComponent.SetMaterial` _returnvalue 0 _returnvalue_2)
      (bind _returnvalue_3 (`|GetDataTableRow` "/Game/DT_ColorTable.DT_ColorTable" "Left")
        (:`then`
          (`MaterialInstanceDynamic.SetVectorParameterValue` _returnvalue_2 "Color" (`.Color_2_CFD72002491B7286ABA2E1915FB5A22F` (break `/Game/S_SideColor` _returnvalue_3))))))
    (:`1`
      _)
    (:`2`
      (bind _returnvalue_4 (`AddComponent|NODE_AddStaticMeshComponent-1`))
      (`StaticMeshComponent.SetStaticMesh` _returnvalue_4 "/Game/Meshes/cubie_seg.cubie_seg")
      (`SceneComponent.K2_SetRelativeTransform` _returnvalue_4 (`KismetMathLibrary.MakeTransform` (100.0 0.0 0.0) (struct :`Pitch` -90.0) (0.86 0.86 0.86)) false false)
      (bind _returnvalue_5 (`PrimitiveComponent.CreateDynamicMaterialInstance` _returnvalue_4 0 "/Game/MT_Side.MT_Side" "None"))
      (`KismetArrayLibrary.Array_Add` (`self.SideMaterials`) _returnvalue_5)
      (`PrimitiveComponent.SetMaterial` _returnvalue_4 0 _returnvalue_5)
      (bind _returnvalue_6 (`|GetDataTableRow` "/Game/DT_ColorTable.DT_ColorTable" "Right")
        (:`then`
          (`MaterialInstanceDynamic.SetVectorParameterValue` _returnvalue_5 "Color" (`.Color_2_CFD72002491B7286ABA2E1915FB5A22F` (break `/Game/S_SideColor` _returnvalue_6)))))))
  (switch `int` (`|GetArrayItem` _initcubeindex 1)
    (:`0`
      (bind _returnvalue_7 (`AddComponent|NODE_AddStaticMeshComponent-2`))
      (`StaticMeshComponent.SetStaticMesh` _returnvalue_7 "/Game/Meshes/cubie_seg.cubie_seg")
      (`SceneComponent.K2_SetRelativeTransform` _returnvalue_7 (`KismetMathLibrary.MakeTransform` (0.0 -100.0 0.0) (struct :`Roll` 90.0) (0.86 0.86 0.86)) false false)
      (bind _returnvalue_8 (`PrimitiveComponent.CreateDynamicMaterialInstance` _returnvalue_7 0 "/Game/MT_Side.MT_Side" "None"))
      (`KismetArrayLibrary.Array_Add` (`self.SideMaterials`) _returnvalue_8)
      (`PrimitiveComponent.SetMaterial` _returnvalue_7 0 _returnvalue_8)
      (bind _returnvalue_9 (`|GetDataTableRow` "/Game/DT_ColorTable.DT_ColorTable" "Back")
        (:`then`
          (`MaterialInstanceDynamic.SetVectorParameterValue` _returnvalue_8 "Color" (`.Color_2_CFD72002491B7286ABA2E1915FB5A22F` (break `/Game/S_SideColor` _returnvalue_9))))))
    (:`1`
      _)
    (:`2`
      (bind _returnvalue_10 (`AddComponent|NODE_AddStaticMeshComponent-3`))
      (`StaticMeshComponent.SetStaticMesh` _returnvalue_10 "/Game/Meshes/cubie_seg.cubie_seg")
      (`SceneComponent.K2_SetRelativeTransform` _returnvalue_10 (`KismetMathLibrary.MakeTransform` (0.0 100.0 0.0) (struct :`Roll` -90.0) (0.86 0.86 0.86)) false false)
      (bind _returnvalue_11 (`PrimitiveComponent.CreateDynamicMaterialInstance` _returnvalue_10 0 "/Game/MT_Side.MT_Side" "None"))
      (`KismetArrayLibrary.Array_Add` (`self.SideMaterials`) _returnvalue_11)
      (`PrimitiveComponent.SetMaterial` _returnvalue_10 0 _returnvalue_11)
      (bind _returnvalue_12 (`|GetDataTableRow` "/Game/DT_ColorTable.DT_ColorTable" "Front")
        (:`then`
          (`MaterialInstanceDynamic.SetVectorParameterValue` _returnvalue_11 "Color" (`.Color_2_CFD72002491B7286ABA2E1915FB5A22F` (break `/Game/S_SideColor` _returnvalue_12)))))))
  (switch `int` (`|GetArrayItem` _initcubeindex 2)
    (:`0`
      (bind _returnvalue_13 (`AddComponent|NODE_AddStaticMeshComponent-4`))
      (`StaticMeshComponent.SetStaticMesh` _returnvalue_13 "/Game/Meshes/cubie_seg.cubie_seg")
      (`SceneComponent.K2_SetRelativeTransform` _returnvalue_13 (`KismetMathLibrary.MakeTransform` (0.0 0.0 -100.0) (struct) (0.86 0.86 0.86)) false false)
      (bind _returnvalue_14 (`PrimitiveComponent.CreateDynamicMaterialInstance` _returnvalue_13 0 "/Game/MT_Side.MT_Side" "None"))
      (`KismetArrayLibrary.Array_Add` (`self.SideMaterials`) _returnvalue_14)
      (`PrimitiveComponent.SetMaterial` _returnvalue_13 0 _returnvalue_14)
      (bind _returnvalue_15 (`|GetDataTableRow` "/Game/DT_ColorTable.DT_ColorTable" "Bottom")
        (:`then`
          (`MaterialInstanceDynamic.SetVectorParameterValue` _returnvalue_14 "Color" (`.Color_2_CFD72002491B7286ABA2E1915FB5A22F` (break `/Game/S_SideColor` _returnvalue_15))))))
    (:`2`
      (bind _returnvalue_16 (`AddComponent|NODE_AddStaticMeshComponent-5`))
      (`StaticMeshComponent.SetStaticMesh` _returnvalue_16 "/Game/Meshes/cubie_seg.cubie_seg")
      (`SceneComponent.K2_SetRelativeTransform` _returnvalue_16 (`KismetMathLibrary.MakeTransform` (0.0 0.0 100.0) (struct) (0.86 0.86 0.86)) false false)
      (bind _returnvalue_17 (`PrimitiveComponent.CreateDynamicMaterialInstance` _returnvalue_16 0 "/Game/MT_Side.MT_Side" "None"))
      (`KismetArrayLibrary.Array_Add` (`self.SideMaterials`) _returnvalue_17)
      (`PrimitiveComponent.SetMaterial` _returnvalue_16 0 _returnvalue_17)
      (bind _returnvalue_18 (`|GetDataTableRow` "/Game/DT_ColorTable.DT_ColorTable" "Top")
        (:`then`
          (`MaterialInstanceDynamic.SetVectorParameterValue` _returnvalue_17 "Color" (`.Color_2_CFD72002491B7286ABA2E1915FB5A22F` (break `/Game/S_SideColor` _returnvalue_18))))))))

(fn `SetMaterialEmission`
  (params (Intensity :type "Float (double-precision)"))
  (for _array_element (`self.SideMaterials`)
    (`MaterialInstanceDynamic.SetScalarParameterValue` _array_element "Intensity" (* Intensity 10.0))))

(fn `UserConstructionScript`)